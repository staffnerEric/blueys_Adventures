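; BP_PlayerControler is a player controller Blueprint that handles player death and restarts the game.
; Its onDeath event unpossesses the pawn, fades the camera out and holds the fade, then shows a Died widget.
; After a short delay it removes the widget and calls RestartGame on the GameMode.
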(event Custom|on%20Death
  (Pawn|UnPossess)
  (CameraFades|StartCameraFade :self (Variables|Default|GetPlayerCameraManager) :ToAlpha 1.0 :Duration 1.0 :bHoldWhenFinished true)
  (bind _returnvalue (UserInterface|CreateWidget "/Game/BP/died.died_C" self))
  (UserInterface|Viewport|AddtoViewport _returnvalue 0)
  (Utilities|FlowControl|Delay 2.0)
  (Widget|RemovefromParent _returnvalue)
  (bind _asgame_mode (Utilities|Casting|CastToGameMode (Game|GetGameMode)))
  (Class|GameMode|RestartGame _asgame_mode))

(event EventBeginPlay)

(event EventTick
  (params (DeltaSeconds :type Float%20%28single-precision%29)))

(fn ConstructionScript)